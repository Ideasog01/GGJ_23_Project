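; Player character Blueprint that handles sprinting, survival stats, pausing and death.
; Sprint input swaps walk speed and runs looping timers that drain Energy while held and refill it on release.
; Tick uses Delays to throttle Food and Thirst decay, draining Health when either runs out and opening DeathMenu at zero Health.
; PauseGame toggles a cached PauseMenu widget, game pause, cursor and input mode while Health remains.
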(event Custom|PlayerSprint
  ;[1 1 1] Sprint Mechanic
  (Utilities|Time|ClearandInvalidateTimerbyHandle (stale Custom|StopSprint _returnvalue))
  (Variables|/Script/Engine.CharacterMovementComponent|SetMaxWalkSpeed (Variables|Character|GetCharacterMovement) 1e+03)
  (bind _returnvalue (Utilities|Time|SetTimerbyEvent (delegate Custom|PlayerSprint) 0.2 true))
  (if (<= (Variables|Default|GetEnergy) 0.0)
    (CallFunction|StopSprint)
    (else
      (Variables|Default|SetEnergy (- (Variables|Default|GetEnergy) 1.0)))))

(event Custom|StopSprint
  ;[1 1 1] Sprint Mechanic
  (Utilities|Time|ClearandInvalidateTimerbyHandle (stale Custom|PlayerSprint _returnvalue))
  (Variables|/Script/Engine.CharacterMovementComponent|SetMaxWalkSpeed (Variables|Character|GetCharacterMovement) 6e+02)
  (bind _returnvalue (Utilities|Time|SetTimerbyEvent (delegate Custom|StopSprint) 0.2 true))
  (if (>= (Variables|Default|GetEnergy) 1e+02)
    (Utilities|Time|ClearandInvalidateTimerbyHandle _returnvalue)
    (else
      (Variables|Default|SetEnergy (+ (Variables|Default|GetEnergy) 1.0)))))

(event EventTick
  (params (DeltaSeconds :type Float%20%28single-precision%29))
  ;[1 1 1] Decrease Hunger & Thirst
  (Class|AutomationBlueprintFunctionLibrary|AutomationWaitforLoading)
  (Utilities|FlowControl|Sequence
    (:then_0
      (if (> (Variables|Default|GetFood) 0.0)
        (Utilities|FlowControl|Delay 1.0)
        (Variables|Default|SetFood (- (Variables|Default|GetFood) 0.2))
        (else
          (if (> (Variables|Default|GetHealth) 0.0) :!label _label
            (Utilities|FlowControl|Delay 1.0)
            (Variables|Default|SetHealth (- (Variables|Default|GetHealth) 0.2))))))
    (:then_1
      (if (> (Variables|Default|GetThirst) 0.0)
        (Utilities|FlowControl|Delay 1.5)
        (Variables|Default|SetThirst (- (Variables|Default|GetThirst) 0.3))
        (else
          (goto _label))))
    (:then_2
      (if (<= (Variables|Default|GetHealth) 0.0)
        (Viewport|RemoveAllWidgets)
        (Game|OpenLevel(byName) "DeathMenu")))))

(event Input|ActionEvents|InputActionPauseGame
  (params (Key :type Key%20Structure :default "None"))
  (bind _returnvalue (Game|GetPlayerController 0))
  ;[1 1 1] Pause/ Unpause Game ( Input P / ESC )
  (:Pressed
    (if (> (Variables|Default|GetHealth) 0.0)
      (Utilities|IsValid (Variables|Default|GetPause%20Menu%20REF)
        (:Is%20Valid
          _)
        (:Is%20Not%20Valid
          (bind _returnvalue_2 (UserInterface|CreateWidget "/Game/HUD/PauseMenu.PauseMenu_C"))
          (Variables|Default|SetPause%20Menu%20REF _returnvalue_2)))
      (if (Game|IsGamePaused)
        (Widget|RemovefromParent (Variables|Default|GetPause%20Menu%20REF))
        (Game|SetGamePaused false)
        (Variables|/Script/Engine.PlayerController|SetbShowMouseCursor _returnvalue false)
        (Input|SetInputModeGameOnly _returnvalue)
        (else
          (UserInterface|Viewport|AddtoViewport (Variables|Default|GetPause%20Menu%20REF) 0)
          (Game|SetGamePaused true)
          (Variables|/Script/Engine.PlayerController|SetbShowMouseCursor _returnvalue true)
          (Input|SetInputModeGameandUI _returnvalue (Variables|Default|GetPause%20Menu%20REF) "LockInFullscreen" false))))))

(event Input|ActionEvents|InputActionSprint
  (params (Key :type Key%20Structure :default "None"))
  ;[1 1 1] Sprint Mechanic
  (:Pressed
    (CallFunction|PlayerSprint))
  (:Released
    (CallFunction|StopSprint)))

(fn ConstructionScript)