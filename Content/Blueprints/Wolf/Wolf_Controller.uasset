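; Wolf_Controller is the AI controller for the wolf enemy, running the Wolf_BT behavior tree on BeginPlay.
; AI perception updates set the HasSpottedPlayer blackboard key to whether the player is currently sensed.
; Every tick, it sets IsNear from whether the player pawn is within a short fixed distance of the controlled wolf.
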(event OnTargetPerceptionUpdated(AIPerception)
  (params (Actor :type Actor%20Object%20Reference) (Stimulus :type AI%20Stimulus%20Structure))
  (Utilities|Casting|CastToPlayer_BP Actor)
  (AI|Components|Blackboard|SetValueasBool (AI|GetBlackboard 0) (Utilities|Name|MakeLiteralName "HasSpottedPlayer") (.bSuccessfullySensed (Utilities|Struct|BreakAIStimulus Stimulus))))

(event EventTick
  (params (DeltaSeconds :type Float%20%28single-precision%29))
  (AI|Components|Blackboard|SetValueasBool (AI|GetBlackboard 0) (Utilities|Name|MakeLiteralName "IsNear") (< (Math|Vector|Distance(Vector) (Transformation|GetActorLocation (Game|Player|GetPlayerPawn 0)) (Transformation|GetActorLocation (Pawn|GetControlledPawn))) 2e+02)))

(event EventBeginPlay
  (AI|RunBehaviorTree "/Game/Blueprints/Wolf/Wolf_BT.Wolf_BT"))

(fn ConstructionScript)